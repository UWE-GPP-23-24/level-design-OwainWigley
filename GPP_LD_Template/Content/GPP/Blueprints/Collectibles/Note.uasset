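; Collectible note actor that offers an interact prompt on overlap and hands its text to the player character.
; BeginPlay caches the player and runs NoteText through FormatText to substitute its /n placeholder.
; Any overlap shows a SignInteract widget, enables player interaction and passes the text, a self reference and a destroy flag through GetText.
; Ending overlap removes the prompt and disables interaction, while RemoveInteractUI also removes the prompt.
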(event `RemoveInteractUI`
  (`Widget.RemoveFromParent` (`self.InteractReference`)))

(event `self.ReceiveBeginPlay`
  (bind _returnvalue (`GameplayStatics.GetActorOfClass` "/Game/GPP/Blueprints/Essential/BP_PlayerCharacter.BP_PlayerCharacter_C"))
  (set `self.PlayerReference` _returnvalue)
  (set `self.NoteText` (`|FormatText` (`self.NoteText`) " \n")))

(event `self.ReceiveActorBeginOverlap`
  (params (OtherActor :type "Actor Object Reference"))
  (bind _returnvalue (`|CreateWidget` "/Game/GPP/Widgets/HUD/SignInteract.SignInteract_C"))
  (bind _output_get (set `self.InteractReference` _returnvalue))
  (`UserWidget.AddToViewport` _output_get 0)
  (set `/Game/GPP/Blueprints/Essential/BP_PlayerCharacter.CanInteract` true (`self.PlayerReference`))
  (`/Game/GPP/Blueprints/Essential/BP_PlayerCharacter.GetText` (`self.PlayerReference`) (`self.NoteText`) true self null))

(event `self.ReceiveActorEndOverlap`
  (params (OtherActor :type "Actor Object Reference"))
  (`Widget.RemoveFromParent` (`self.InteractReference`))
  (set `/Game/GPP/Blueprints/Essential/BP_PlayerCharacter.CanInteract` false (`self.PlayerReference`)))

(fn `UserConstructionScript`)