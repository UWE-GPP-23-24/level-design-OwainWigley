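; Collectible key pickup that spins in place and increments the player's key count on overlap.
; Pickup removes the trigger box, freezes the player's input and movement, turns them toward the key and briefly shows a collected widget.
; Tutorial keys then notify CheckKeysVolume, while other keys teleport the player to that volume behind a fade to black.
; The key destroys itself afterward, leaving input restoration to logic outside this Blueprint.
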(event `self.ReceiveBeginPlay`
  (bind _returnvalue (`GameplayStatics.GetActorOfClass` "/Game/GPP/Blueprints/Essential/BP_PlayerCharacter.BP_PlayerCharacter_C"))
  (set `self.PlayerReference` _returnvalue))

(event `self.ReceiveActorBeginOverlap`
  (params (OtherActor :type "Actor Object Reference"))
  (bind _playerreference (`self.PlayerReference`))
  (`ActorComponent.K2_DestroyComponent` (`self.Box`))
  (set `/Game/GPP/Blueprints/Essential/BP_PlayerCharacter.KeysCollected` (+ (`/Game/GPP/Blueprints/Essential/BP_PlayerCharacter.KeysCollected` _playerreference) 1) _playerreference)
  (set `/Game/GPP/Blueprints/Essential/BP_PlayerCharacter.CanUseInput` false (`self.PlayerReference`))
  (`MovementComponent.StopMovementImmediately` (`Character.CharacterMovement` (`self.PlayerReference`)))
  (`/Game/GPP/Blueprints/Essential/LookAtInterface.LookAt` (`self.PlayerReference`) self 0.0 0.0 0.0)
  (bind _returnvalue (`|CreateWidget` "/Game/GPP/Widgets/HUD/KeyCollected.KeyCollected_C"))
  (bind _output_get (set `self.KeyCollectedReference` _returnvalue))
  (`UserWidget.AddToViewport` _output_get 0)
  (`KismetSystemLibrary.Delay` 2.0)
  (`Widget.RemoveFromParent` (`self.KeyCollectedReference`))
  (if (`self.TutKey`)
    (bind _returnvalue_2 (`GameplayStatics.GetActorOfClass` "/Game/GPP/Blueprints/KeyProgression/CheckKeysVolume.CheckKeysVolume_C"))
    (`/Game/GPP/Blueprints/KeyProgression/CheckKeysVolume.TutKey` _returnvalue_2)
    (else
      (bind _returnvalue_3 (`|CreateWidget` "/Game/GPP/Widgets/FadeToBlackWidget.FadeToBlackWidget_C"))
      (bind _output_get_2 (set `self.FadeReference` _returnvalue_3))
      (`UserWidget.AddToViewport` _output_get_2 0)
      (`KismetSystemLibrary.Delay` 1.0)
      (bind _returnvalue_4 (`GameplayStatics.GetActorOfClass` "/Game/GPP/Blueprints/KeyProgression/CheckKeysVolume.CheckKeysVolume_C"))
      (`self.K2_SetActorLocation` (`self.PlayerReference`) (`self.K2_GetActorLocation` _returnvalue_4) false true)
      (`/Game/GPP/Widgets/FadeToBlackWidget.FadeOut` (`self.FadeReference`))
      (`KismetSystemLibrary.Delay` 1.0)
      (`Widget.RemoveFromParent` (`self.FadeReference`))))
  (`self.K2_DestroyActor`))

(event `self.ReceiveTick`
  (params (DeltaSeconds :type "Float (single-precision)"))
  (`self.K2_AddActorWorldRotation` (`KismetMathLibrary.MakeRotator` 0.0 0.0 (* DeltaSeconds (`self.RotateSpeed`)))))

(fn `UserConstructionScript`)