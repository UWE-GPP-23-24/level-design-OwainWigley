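; BP_CoinBox is a breakable collectible box that spawns three BP_Coin actors and then destroys itself.
; It breaks through either the BreakBox event or any overlap with its Box1 component.
; The coins appear in a row along world X, centered on the box and inheriting its rotation and scale.
; Floating boxes lower the coins by SpawnOffset, while others zero that offset.
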(event `BreakBox`
  (bind _rotation (.rotation (`self.GetTransform`)))
  (bind _scale (.scale (`self.GetTransform`)))
  (bind _x (.x (.location (`self.GetTransform`))))
  (bind _y (.y (.location (`self.GetTransform`))))
  (bind _returnvalue (- (.z (.location (`self.GetTransform`))) (`self.SpawnOffset`)))
  (if (not (`self.Floating`)) :!label _label
    (set `self.SpawnOffset` 0))
  (`|SpawnActorFromClass` "/Game/GPP/Blueprints/Collectibles/BP_Coin.BP_Coin_C" (`KismetMathLibrary.MakeTransform` (`KismetMathLibrary.MakeVector` _x _y _returnvalue) _rotation _scale) "Undefined" "MultiplyWithRoot" null null)
  (`|SpawnActorFromClass` "/Game/GPP/Blueprints/Collectibles/BP_Coin.BP_Coin_C" (`KismetMathLibrary.MakeTransform` (`KismetMathLibrary.MakeVector` (+ _x 75.0) _y _returnvalue) _rotation _scale) "Undefined" "MultiplyWithRoot" null null)
  (`|SpawnActorFromClass` "/Game/GPP/Blueprints/Collectibles/BP_Coin.BP_Coin_C" (`KismetMathLibrary.MakeTransform` (`KismetMathLibrary.MakeVector` (- _x 75.0) _y _returnvalue) _rotation _scale) "Undefined" "MultiplyWithRoot" null null)
  (`self.K2_DestroyActor`))

(event `self.Box1.OnComponentBeginOverlap`
  (params (OverlappedComponent :type "PrimitiveComponent Object Reference") (OtherActor :type "Actor Object Reference") (OtherComp :type "PrimitiveComponent Object Reference") (OtherBodyIndex :type Integer) (bFromSweep :type Boolean) (SweepResult :type "HitResult Structure (by ref)"))
  (goto _label))

(fn `UserConstructionScript`)