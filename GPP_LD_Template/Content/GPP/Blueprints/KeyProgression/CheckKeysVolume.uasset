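; CheckKeysVolume is a key-progression trigger that opens the Gate once the player has collected at least three keys.
; An actor overlap or the TutKey event runs the same check on the BP_PlayerCharacter found by class lookup, without filtering the overlapping actor.
; On success it calls Collapse on the Gate, waits briefly, enables player input and destroys itself.
; Otherwise it just enables player input.
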(event `self.ReceiveActorBeginOverlap`
  (params (OtherActor :type "Actor Object Reference"))
  (bind _returnvalue (`GameplayStatics.GetActorOfClass` "/Game/GPP/Blueprints/Essential/BP_PlayerCharacter.BP_PlayerCharacter_C" :!label _label))
  (set `self.PlayerReference` _returnvalue)
  (if (>= (`/Game/GPP/Blueprints/Essential/BP_PlayerCharacter.KeysCollected` (`self.PlayerReference`)) 3)
    (bind _returnvalue_2 (`GameplayStatics.GetActorOfClass` "/Game/GPP/Blueprints/KeyProgression/Gate.Gate_C"))
    (`/Game/GPP/Blueprints/KeyProgression/Gate.Collapse` _returnvalue_2)
    (`KismetSystemLibrary.Delay` 1.0)
    (set `/Game/GPP/Blueprints/Essential/BP_PlayerCharacter.CanUseInput` true (`self.PlayerReference`))
    (`self.K2_DestroyActor`)
    (else
      (set `/Game/GPP/Blueprints/Essential/BP_PlayerCharacter.CanUseInput` true (`self.PlayerReference`)))))

(event `TutKey`
  (goto _label))

(fn `UserConstructionScript`)