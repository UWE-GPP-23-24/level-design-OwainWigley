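; Key progression gate actor that, when Collapse is called, opens the way by dropping its door and revealing coins.
; Collapse makes the player character look at the gate, turns the Door into a non-colliding physics body and destroys the linked blocking volumes.
; After a delay it unhides the first five Coins one at a time through staggered delays, then destroys itself.
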(event `Collapse`
  (bind _returnvalue (`GameplayStatics.GetActorOfClass` "/Game/GPP/Blueprints/Essential/BP_PlayerCharacter.BP_PlayerCharacter_C"))
  (`/Game/GPP/Blueprints/Essential/LookAtInterface.LookAt` _returnvalue self 0.0 0.0 0.0)
  (`PrimitiveComponent.SetCollisionResponseToAllChannels` (`self.Door`) "ECR_Ignore")
  (`PrimitiveComponent.SetSimulatePhysics` (`self.Door`) true)
  (for _array_element (`self.BlockingVolumes`)
    (`self.K2_DestroyActor` _array_element))
  (`KismetSystemLibrary.Delay` 1.3)
  (for (_array_element_2 _array_index) (`self.Coins`)
    (if (== _array_index 0)
      (`self.SetActorHiddenInGame` _array_element_2 false)))
  (`KismetSystemLibrary.Delay` 0.3)
  (for (_array_element_3 _array_index_2) (`self.Coins`)
    (if (== _array_index_2 1)
      (`self.SetActorHiddenInGame` _array_element_3 false)))
  (`KismetSystemLibrary.Delay` 0.3)
  (for (_array_element_4 _array_index_3) (`self.Coins`)
    (if (== _array_index_3 2)
      (`self.SetActorHiddenInGame` _array_element_4 false)))
  (`KismetSystemLibrary.Delay` 0.3)
  (for (_array_element_5 _array_index_4) (`self.Coins`)
    (if (== _array_index_4 3)
      (`self.SetActorHiddenInGame` _array_element_5 false)))
  (`KismetSystemLibrary.Delay` 0.3)
  (for (_array_element_6 _array_index_5) (`self.Coins`)
    (if (== _array_index_5 4)
      (`self.SetActorHiddenInGame` _array_element_6 false)))
  (`self.K2_DestroyActor`))

(fn `UserConstructionScript`)