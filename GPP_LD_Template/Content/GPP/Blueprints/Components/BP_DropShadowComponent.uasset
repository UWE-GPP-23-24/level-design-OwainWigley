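; Actor component that spawns a drop shadow decal on its owning Character's mesh at BeginPlay, meant to mark the ground beneath airborne characters.
; ShouldShowDecal is true when the character is not moving on ground.
; The update logic toggles visibility, line-traces downward, moves the decal to the hit and shrinks it with distance.
; That update logic is disconnected from the empty Tick, so it never runs.
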(event `self.ReceiveBeginPlay`
  ;[0.4491 0.8591 1] Init Decal
  ;;[0.4491 0.8591 1] Cache player ref
  (bind _ascharacter (cast `Character` (`self.GetOwner`)))
  (bind _output_get (set `self.As Character` _ascharacter))
  ;;[0.4491 0.8591 1] Spawn decal and cache ref
  (bind _returnvalue (`GameplayStatics.SpawnDecalAttached` "/Game/GPP/Materials/M_DecalDropShadow.M_DecalDropShadow" (5.0 60.0 60.0) (`Character.Mesh` _output_get) "None" (0.0 0.0 0.0) (struct :`Pitch` 90.0)))
  (set `self.DropDecal` _returnvalue))

(event `self.ReceiveTick`
  (params (DeltaSeconds :type "Float (single-precision)")))

(fn `ShouldShowDecal`
  (returns (ReturnValue :type Boolean))
  (return (not (`NavMovementComponent.IsMovingOnGround` (`Character.CharacterMovement` (`self.As Character`))))))